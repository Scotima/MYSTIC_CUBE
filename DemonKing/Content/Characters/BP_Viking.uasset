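; Viking character Blueprint that carries out the Q skill, a melee-style attack.
; UseSkillQ prints a debug string, plays the attack montage, then uses fixed delays to time PerformSkillQHitCheck and clear the casting flag afterward.
; The hit check and casting setter are called here but defined outside this file.
; Movement input events are empty, with camera-yaw movement and hand-trail Niagara nodes left disconnected.
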(event EventBeginPlay)

(event Collision|EventActorBeginOverlap
  (params (OtherActor :type Actor%20Object%20Reference)))

(event EventTick
  (params (DeltaSeconds :type Float%20%28single-precision%29)))

(event EventUseSkillQ
  (Development|PrintString "Use Skill Q")
  (Animation|PlayAnimMontage "/Game/Viking/Animations/Anim_Viking_attack2_Montage.Anim_Viking_attack2_Montage" 1.0 "None")
  (Utilities|FlowControl|Delay 0.15)
  (Class|PlayerCharacterBase|PerformSkillQHitCheck)
  (Utilities|FlowControl|Delay 0.2)
  (Class|PlayerCharacterBase|SetCastingSkill false))

(event Input|AxisEvents|InputAxisMoveForward
  (params (AxisValue :type Float%20%28single-precision%29)))

(event Input|AxisEvents|InputAxisMoveRight
  (params (AxisValue :type Float%20%28single-precision%29)))

(fn ConstructionScript)