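; Menu player character that spawns a rotatable display character and lets the mouse spin it.
; On BeginPlay it finds a BP_ReusableLocationMarker, switches on its Type and spawns BP_RotableCharacter at that marker's transform, keeping a reference.
; Horizontal mouse input applies inverted, scaled world yaw to the spawned character while CanRotateCharacter is true, a flag exposed through a setter function.
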(event EventBeginPlay
  ;[0.15 0.15 0.15 0.5] Spawn Rotable Character Once MenuPlayerCharacter is ready
  (bind _returnvalue (Actor|GetActorOfClass "/Game/ModularShowcase/Blueprints/BP_ReusableLocationMarker.BP_ReusableLocationMarker_C"))
  (switch Utilities|FlowControl|Switch|SwitchonE_ReusableSpawnerType (Variables|/Game/ModularShowcase/Blueprints/BP_ReusableLocationMarker.BP_ReusableLocationMarker_C|GetType _returnvalue)
    (:NewEnumerator0
      (bind _returnvalue_2 (Game|SpawnActorfromClass "/Game/ModularShowcase/Blueprints/BP_RotableCharacter.BP_RotableCharacter_C" (Math|Transform|MakeTransform (Transformation|GetActorLocation _returnvalue) (Transformation|GetActorRotation _returnvalue) "1.000000,1.000000,1.000000") "AdjustIfPossibleButAlwaysSpawn" "MultiplyWithRoot" 0 0))
      (Variables|Default|SetSpawnedRotableCharRef _returnvalue_2))))

(event Input|MouseEvents|MouseX
  (params (AxisValue :type Float%20%28single-precision%29))
  ;[0.15 0.15 0.15 0.5] Display Character Rotation
  (if (Variables|Default|GetCanRotateCharacter)
    (Class|Actor|AddActorWorldRotation (Variables|Default|GetSpawnedRotableCharRef) (Math|Rotator|MakeRotator 0.0 0.0 (* AxisValue -5.0)))))

(fn ConstructionScript)

(fn SetCanRotateCharacter
  (params (CanRotateCharacter :type Boolean))
  (Variables|Default|SetCanRotateCharacter CanRotateCharacter))