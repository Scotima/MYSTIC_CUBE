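; Blueprint function library of global shortcuts for the modular showcase's main menu, covering character rotation, notifications, currency purchases and the player name.
; Each function fetches a framework object, casts it to its showcase class and forwards the call, stopping if the cast fails.
; Rotation and currency go through the first player's menu character, notifications through the game mode's main menu widget, and the name through the game instance.
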(fn SetCanRotateCharacter
  (params (CanRotateCharacter :type Boolean))
  (bind _asbp_menu_player_character (Utilities|Casting|CastToBP_MenuPlayerCharacter (Game|Player|GetPlayerPawn 0)))
  (Default|SetCanRotateCharacter _asbp_menu_player_character CanRotateCharacter))

(fn SendNotification
  (params (NotificationType :type E_NotificationType%20Enum :default "NewEnumerator0") (NotificationMessage :type String))
  (bind _asbp_main_menu_game_mode (Utilities|Casting|CastToBP_MainMenuGameMode (Game|GetGameMode)))
  (Default|SendNotification (Variables|/Game/ModularShowcase/Blueprints/BP_MainMenuGameMode.BP_MainMenuGameMode_C|GetMain%20Menu%20Widget%20Ref _asbp_main_menu_game_mode) NotificationType NotificationMessage))

(fn BuyItem
  (params (CurrencyType :type E_CurrencyType%20Enum :default "NewEnumerator0") (ItemPrice :type Integer))
  (bind _asbp_menu_player_character (Utilities|Casting|CastToBP_MenuPlayerCharacter (Game|Player|GetPlayerPawn 0)))
  (bind (_new_currency_valye _was_buying_succesfull) (Default|BuyItem (Variables|/Game/ModularShowcase/Blueprints/BP_MenuPlayerCharacter.BP_MenuPlayerCharacter_C|GetBPC_CurrencyComponent _asbp_menu_player_character) CurrencyType ItemPrice))
  (return _new_currency_valye _was_buying_succesfull))

(fn GetCurrencyComponent
  (bind _asbp_menu_player_character (Utilities|Casting|CastToBP_MenuPlayerCharacter (Game|Player|GetPlayerPawn 0)))
  (return (Variables|/Game/ModularShowcase/Blueprints/BP_MenuPlayerCharacter.BP_MenuPlayerCharacter_C|GetBPC_CurrencyComponent _asbp_menu_player_character)))

(fn GetPlayerName
  (bind _asbp_showcase_instance (Utilities|Casting|CastToBP_ShowcaseInstance (Game|GetGameInstance)))
  (return (Default|GetPlayerName _asbp_showcase_instance)))

(fn SetPlayerName
  (params (PlayerName :type String))
  (bind _asbp_showcase_instance (Utilities|Casting|CastToBP_ShowcaseInstance (Game|GetGameInstance)))
  (Default|SetPlayerName _asbp_showcase_instance PlayerName))