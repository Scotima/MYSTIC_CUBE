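; Currency component that tracks two balances, GG and PRM, with functions to get, set, add, remove and spend currency by type.
; BuyItem checks the balance before deducting and reports success, while RemoveCurrency subtracts without a check.
; Purchases, failed purchases, additions and removals fire event dispatchers.
; When EnableNotifications is set, BeginPlay binds those dispatchers to events that send typed notification messages.
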(event Custom|SendOnItemBoughtNotification
  (CallFunction|SendNotification "NewEnumerator1" "Item Succesfully Bought!"))

(event Custom|SendOnNotEnoughCurrency
  (CallFunction|SendNotification "NewEnumerator2" "Not Enough Currency!"))

(event Custom|SendOnAddedCurrency
  (CallFunction|SendNotification "NewEnumerator1" "Currency Succesfully Added!"))

(event Custom|SendOnCurrencyRemoved
  (CallFunction|SendNotification "NewEnumerator0" "Currency Updated!"))

(event EventBeginPlay
  (if (Variables|Default|GetEnableNotifications)
    (EventDispatchers|BindEventtoOnItemBought (EventDispatchers|CreateEvent :!event Custom|SendOnItemBoughtNotification))
    (EventDispatchers|BindEventtoOnNotEnoughCurrency (EventDispatchers|CreateEvent :!event Custom|SendOnNotEnoughCurrency))
    (EventDispatchers|BindEventtoOnAddedCurrency (EventDispatchers|CreateEvent :!event Custom|SendOnAddedCurrency))
    (EventDispatchers|BindEventtoOnRemovedCurrency (EventDispatchers|CreateEvent :!event Custom|SendOnCurrencyRemoved))))

(fn GetCurrentCurrencyValue
  (params (CurrencyType :type E_CurrencyType%20Enum :default "NewEnumerator0"))
  (switch Utilities|FlowControl|Switch|SwitchonE_CurrencyType CurrencyType
    (:NewEnumerator0
      (return (Variables|Default|GetCurrentGG)))
    (:NewEnumerator1
      (return (Variables|Default|GetCurrentPRM)))))

(fn SetNewCurrentCurrencyValue
  (params (Currency%20Type :type E_CurrencyType%20Enum :default "NewEnumerator0") (New%20Currency%20Value :type Integer))
  (switch Utilities|FlowControl|Switch|SwitchonE_CurrencyType Currency%20Type
    (:NewEnumerator0
      (Variables|Default|SetCurrentGG New%20Currency%20Value))
    (:NewEnumerator1
      (Variables|Default|SetCurrentPRM New%20Currency%20Value))))

(fn BuyItem
  (params (CurrencyType :type E_CurrencyType%20Enum :default "NewEnumerator0") (ItemPrice :type Integer))
  (LocalVariables|SetSavedItemPrice ItemPrice)
  (switch Utilities|FlowControl|Switch|SwitchonE_CurrencyType CurrencyType
    (:NewEnumerator0
      (if (>= (Variables|Default|GetCurrentGG) ItemPrice)
        (bind _output_get (Variables|Default|SetCurrentGG (- (Variables|Default|GetCurrentGG) (LocalVariables|GetSavedItemPrice))))
        (Default|CallOnItemBought)
        (Default|CallOnRemovedCurrency)
        (return _output_get true)
        (else
          (Default|CallOnNotEnoughCurrency)
          (return (Variables|Default|GetCurrentGG) false))))
    (:NewEnumerator1
      (if (>= (Variables|Default|GetCurrentPRM) ItemPrice)
        (bind _output_get_2 (Variables|Default|SetCurrentPRM (- (Variables|Default|GetCurrentPRM) (LocalVariables|GetSavedItemPrice))))
        (Default|CallOnItemBought)
        (Default|CallOnRemovedCurrency)
        (return _output_get_2 true)
        (else
          (Default|CallOnNotEnoughCurrency)
          (return (Variables|Default|GetCurrentPRM) false))))))

(fn AddCurrency
  (params (Currency%20Type :type E_CurrencyType%20Enum :default "NewEnumerator0") (Value%20to%20add :type Integer))
  (LocalVariables|SetCurrency%20Value%20To%20Add Value%20to%20add)
  (switch Utilities|FlowControl|Switch|SwitchonE_CurrencyType Currency%20Type
    (:NewEnumerator0
      (bind _output_get (Variables|Default|SetCurrentGG (+ (Variables|Default|GetCurrentGG) (LocalVariables|GetCurrency%20Value%20To%20Add))))
      (Default|CallOnAddedCurrency)
      (return _output_get))
    (:NewEnumerator1
      (bind _output_get_2 (Variables|Default|SetCurrentPRM (+ (Variables|Default|GetCurrentPRM) (LocalVariables|GetCurrency%20Value%20To%20Add))))
      (Default|CallOnAddedCurrency)
      (return _output_get_2))))

(fn RemoveCurrency
  (params (Currency%20Type :type E_CurrencyType%20Enum :default "NewEnumerator0") (Value%20to%20remove :type Integer))
  (LocalVariables|SetCurrency%20Value%20To%20Remove Value%20to%20remove)
  (switch Utilities|FlowControl|Switch|SwitchonE_CurrencyType Currency%20Type
    (:NewEnumerator0
      (bind _output_get (Variables|Default|SetCurrentGG (- (Variables|Default|GetCurrentGG) (LocalVariables|GetCurrency%20Value%20To%20Remove))))
      (Default|CallOnRemovedCurrency)
      (return _output_get))
    (:NewEnumerator1
      (bind _output_get_2 (Variables|Default|SetCurrentPRM (- (Variables|Default|GetCurrentPRM) (LocalVariables|GetCurrency%20Value%20To%20Remove))))
      (Default|CallOnRemovedCurrency)
      (return _output_get_2))))