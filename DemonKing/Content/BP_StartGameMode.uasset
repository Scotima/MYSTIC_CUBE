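; Game mode that delays spawning a joining player's BP_Viking pawn until there is ground beneath the first PlayerStart.
; PostLogin requires BP_MyGameInstance, then starts a short looping timer that line-traces down through that start point.
; On the first hit, it stops the timer, spawns the Viking high above the impact point, then possesses it and sets it as view target.
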(event Custom|EV_CheckAndSpawn
  (bind (_outhit _returnvalue) (Collision|LineTraceByChannel (+ (.Location (Math|Transform|BreakTransform (Transformation|GetActorTransform (Utilities|Array|Get(acopy) (stale EventPostLogin _outactors))))) "0.000000,0.000000,500.000000") (- (.Location (Math|Transform|BreakTransform (Transformation|GetActorTransform (Utilities|Array|Get(acopy) (stale EventPostLogin _outactors))))) "0.000000,0.000000,5000.000000") "TraceTypeQuery1" false 0 "None"))
  (if _returnvalue
    (Utilities|Time|ClearandInvalidateTimerbyHandle (Variables|Default|GetSpawnTimerHandle))
    (bind _returnvalue_2 (Game|SpawnActorfromClass "/Game/Characters/BP_Viking.BP_Viking_C" (Math|Conversions|ToTransform(Vector) (+ (.ImpactPoint (Collision|BreakHitResult _outhit)) "0.000000,0.000000,3000.000000")) "Undefined" "MultiplyWithRoot" 0 0))
    (Pawn|Possess (stale EventPostLogin NewPlayer) _returnvalue_2)
    (Game|Player|SetViewTargetwithBlend (stale EventPostLogin NewPlayer) _returnvalue_2 0.0 "VTBlend_Linear" 0.0 false)
    (Development|PrintString (Utilities|String|ToString(Vector) (.Location (Math|Transform|BreakTransform (Transformation|GetActorTransform (Utilities|Array|Get(acopy) (stale EventPostLogin _outactors)))))))))

(event EventPostLogin
  (params (NewPlayer :type Player%20Controller%20Object%20Reference))
  (Utilities|Casting|CastToBP_MyGameInstance (Game|GetGameInstance))
  (bind _outactors (Actor|GetAllActorsOfClass "/Script/Engine.PlayerStart"))
  (bind _returnvalue (Utilities|Time|SetTimerbyEvent (delegate Custom|EV_CheckAndSpawn) 0.05 true))
  (Variables|Default|SetSpawnTimerHandle _returnvalue))

(fn ConstructionScript)